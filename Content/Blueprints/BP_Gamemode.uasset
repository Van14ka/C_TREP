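; Game mode for a tile-based runner that builds the track and tracks tile count, score and difficulty.
; On BeginPlay it spawns two tile chains, main and mid, from just below the player start, attaching each tile at the previous one's ConnectionLocationArrow.
; UpdateTileCount increments the count, updates player walk speed, adds score and derives difficulty from every ten tiles.
; Count, score and difficulty changes are broadcast through CallOn events.
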(event EventBeginPlay
  (Utilities|FlowControl|Sequence
    (:then_0
      (bind _output_get (Variables|Default|SetNextTileConnectionTransform (CallFunction|AddZAxisValue (Transformation|GetActorTransform (Class|GameModeBase|FindPlayerStart (Game|GetPlayerController 0))) -1e+02)))
      (Variables|Default|SetNextMidTileConnectionTransform _output_get))
    (:then_1
      (CallFunction|SpawnTile "/Game/Blueprints/Invironment/Tiles/BP_Tile_Start_A.BP_Tile_Start_A_C")
      (for _index (range 0 29)
        (CallFunction|SpawnTile "/Game/Blueprints/Invironment/Tiles/BP_Tile_Main_A.BP_Tile_Main_A_C")))
    (:then_2
      (CallFunction|SpawnMidTile "/Game/Blueprints/Invironment/Tiles/BP_TileMid_Start_A.BP_TileMid_Start_A_C")
      (for _index_2 (range 0 2)
        (CallFunction|SpawnMidTile "/Game/Blueprints/Invironment/BP_TileMidBase.BP_TileMidBase_C")))
    (:then_3
      (CallFunction|UpdateScoreSumm))))

(event EventTick
  (params (DeltaSeconds :type Float%20%28single-precision%29)))

(fn ConstructionScript)

(fn SpawnTile
  (params (InClass :type Actor%20Class%20Reference))
  (bind _returnvalue (Game|SpawnActorfromClass InClass (Variables|Default|GetNextTileConnectionTransform) "Undefined" "MultiplyWithRoot" 0 0))
  (bind _asbp_tile_base (Utilities|Casting|CastToBP_TileBase _returnvalue))
  (Variables|Default|SetNextTileConnectionTransform (Transformation|GetWorldTransform (Variables|/Game/Blueprints/Invironment/BP_TileBase.BP_TileBase_C|GetConnectionLocationArrow _asbp_tile_base))))

(fn SpawnMidTile
  (params (InClass :type Actor%20Class%20Reference))
  (bind _returnvalue (Game|SpawnActorfromClass InClass (Variables|Default|GetNextMidTileConnectionTransform) "Undefined" "MultiplyWithRoot" 0 0))
  (bind _asbp_tile_mid_base (Utilities|Casting|CastToBP_TileMidBase _returnvalue))
  (Variables|Default|SetNextMidTileConnectionTransform (Transformation|GetWorldTransform (Variables|/Game/Blueprints/Invironment/BP_TileMidBase.BP_TileMidBase_C|GetConnectionLocationArrow _asbp_tile_mid_base))))

(fn UpdateTileCount
  (Utilities|FlowControl|Sequence
    (:then_0
      (Math|Integer|IncrementInt (Variables|Default|GetTileCount)
        (:%20%20
          (bind _asbp_player_characters (Utilities|Casting|CastToBP_PlayerCharacters (Game|GetPlayerCharacter 0)))
          (Default|UpdateWalkSpeed _asbp_player_characters true 0.0))))
    (:then_1
      (CallFunction|UpdateScoreSumm (Variables|Default|GetTileScoreMult)))
    (:then_2
      (CallFunction|UpdateCurrentDificulty (/ (Variables|Default|GetTileCount) 10)))
    (:then_3
      (Default|CallOnTileCountUpdated (Variables|Default|GetTileCount)))))

(fn UpdateScoreSumm
  (params (InScore :type Integer))
  (Variables|Default|SetCurrentScore (+ (Variables|Default|GetCurrentScore) InScore))
  (Default|CallOnScoreUpdated (Variables|Default|GetCurrentScore) InScore))

(fn UpdateCurrentDificulty
  (params (InCurrentDificulty :type Integer))
  (Variables|Default|SetCurrentDifficulty InCurrentDificulty)
  (Default|CallOnDifficultyUpdated (Variables|Default|GetCurrentDifficulty)))

(fn AddZAxisValue
  (params (InTransform :type Transform%20%28by%20ref%29) (InZAxisValue :type Float%20%28double-precision%29))
  (bind (_location _rotation _scale) (Math|Transform|BreakTransform InTransform))
  (bind (_x _y _z) (Math|Vector|BreakVector _location))
  (return (Math|Transform|MakeTransform (Math|Vector|MakeVector _x _y (+ _z InZAxisValue)) _rotation _scale)))