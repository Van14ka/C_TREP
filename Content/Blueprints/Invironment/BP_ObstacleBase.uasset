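; Base obstacle actor that kills the player character on contact.
; At BeginPlay it picks a random static mesh from its obstacle mesh array.
; Actor overlaps and mesh hits both cast to the player character and feed one touch function, gated by DoOnce.
; That function triggers the player's death, spawns a puff effect and falling sound, then switches the obstacle mesh to physics simulation.
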(event OnComponentHit(SMC_Obstacle)
  (params (HitComponent :type Primitive%20Component%20Object%20Reference) (OtherActor :type Actor%20Object%20Reference) (OtherComp :type Primitive%20Component%20Object%20Reference) (NormalImpulse :type Vector :default "0, 0, 0") (Hit :type Hit%20Result%20Structure%20%28by%20ref%29))
  (bind _asbp_player_characters (Utilities|Casting|CastToBP_PlayerCharacters OtherActor))
  (Variables|Default|SetCurrent%20Player%20Characters _asbp_player_characters)
  (CallFunction|OnPlayerTouchObstacle))

(event EventBeginPlay
  (CallFunction|UpdateObstacleMeshonRandom))

(event Collision|EventActorBeginOverlap
  (params (OtherActor :type Actor%20Object%20Reference))
  (bind _asbp_player_characters (Utilities|Casting|CastToBP_PlayerCharacters OtherActor))
  (Variables|Default|SetCurrent%20Player%20Characters _asbp_player_characters)
  (CallFunction|OnPlayerTouchObstacle))

(event EventTick
  (params (DeltaSeconds :type Float%20%28single-precision%29)))

(fn ConstructionScript)

(fn UpdateObstacleMeshonRandom
  (if (Utilities|Array|IsValidIndex (Variables|Components|GetObstacleStaticMeshes))
    (Components|StaticMesh|SetStaticMesh (Variables|Default|GetSMC_Obstacle) (Utilities|Array|Get(acopy) (Variables|Components|GetObstacleStaticMeshes) (Math|Random|RandomIntegerinRange 0 (Utilities|Array|LastIndex (Variables|Components|GetObstacleStaticMeshes)))))))

(fn OnPlayerTouchObstacle
  (Utilities|FlowControl|DoOnce false
    (:Completed
      (Default|Death (Variables|Default|GetCurrent%20Player%20Characters))
      (Effects|SpawnEmitteratLocation "/Game/Art/CartoonFX2/Particles/ExplosionParts/PS_SmallPuffs.PS_SmallPuffs" (Transformation|GetWorldLocation (Variables|Default|GetEffectScene)))
      (Audio|SpawnSoundAttached "/Game/Audio/ItemsAndInterfaces/WaveFiles/Cartoon_Falling_05.Cartoon_Falling_05" (Variables|Default|GetDefaultSceneRoot) "None" "0, 0, 0" "0, 0, 0" "KeepRelativeOffset" false 1.0 1.0 0.0 0 0)
      (Collision|SetCollisionProfileName (Variables|Default|GetSMC_Obstacle) "PhysicsActor" true :!class /Script/Engine.PrimitiveComponent)
      (Physics|SetSimulatePhysics (Variables|Default|GetSMC_Obstacle) true))))