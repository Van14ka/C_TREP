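; BP_Bonus_Buff is a bonus Blueprint that applies a walk speed buff to the player character.
; Its ApplyBonus override casts player character 0 to BP_PlayerCharacters and calls UpdateWalkSpeed flagged as an increase, with a step of zero.
; The parent ApplyBonus call is left unconnected, and the event graph holds only disabled default events.
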(event EventBeginPlay
  (|CallParentFunction) ; This node is disabled and will not be called.\nDrag off pins to build functionality.
)

(event Collision|EventActorBeginOverlap
  (params (OtherActor :type Actor%20Object%20Reference))
  (|CallParentFunction OtherActor) ; This node is disabled and will not be called.\nDrag off pins to build functionality.
)

(event EventTick
  (params (DeltaSeconds :type Float%20%28single-precision%29))
  (|CallParentFunction DeltaSeconds) ; This node is disabled and will not be called.\nDrag off pins to build functionality.
)

(fn ConstructionScript
  (|CallParentFunction))

(fn ApplyBonus
  (bind _asbp_player_characters (Utilities|Casting|CastToBP_PlayerCharacters (Game|GetPlayerCharacter 0)))
  (Default|UpdateWalkSpeed _asbp_player_characters true 0.0))