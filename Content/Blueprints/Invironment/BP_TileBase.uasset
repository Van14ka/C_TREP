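; Base track tile for an endless runner that fills its three lanes with random obstacles or bonuses on BeginPlay.
; Difficulty checks against the gamemode's current difficulty gate lane spawns and extra obstacle rolls, and one roll branches into coin or speed pickups.
; When a player overlaps the exit box, it has the gamemode spawn a new tile and update the count, then after a delay destroys itself and its spawned actors.
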(event OnComponentBeginOverlap(TileExitBoxCollision)
  (params (OverlappedComponent :type Primitive%20Component%20Object%20Reference) (OtherActor :type Actor%20Object%20Reference) (OtherComp :type Primitive%20Component%20Object%20Reference) (OtherBodyIndex :type Integer) (bFromSweep :type Boolean) (SweepResult :type Hit%20Result%20Structure%20%28by%20ref%29))
  (Utilities|Casting|CastToBP_PlayerCharacters OtherActor)
  (Default|SpawnTile (Variables|Default|GetCurrentGamemode) "/Game/Blueprints/Invironment/Tiles/BP_Tile_Main_A.BP_Tile_Main_A_C")
  (Default|UpdateTileCount (Variables|Default|GetCurrentGamemode))
  (Utilities|FlowControl|Delay 3.0)
  (CallFunction|TileEnds))

(event EventBeginPlay
  (Utilities|FlowControl|Sequence
    (:then_0
      (bind _asbp_gamemode (Utilities|Casting|CastToBP_Gamemode (Game|GetGameMode)))
      (Variables|Default|SetCurrentGamemode _asbp_gamemode))
    (:then_1
      (CallFunction|SpawnObstacles))))

(fn ConstructionScript)

(fn SpawnObstacles
  (Utilities|FlowControl|Sequence
    (:then_0
      (if (CallFunction|FirstDifficultyCheck)
        (CallFunction|RandomSpawnObstacle (Transformation|GetWorldTransform (Variables|Default|GetLaneArrow_0)))))
    (:then_1
      (if (CallFunction|FirstDifficultyCheck)
        (CallFunction|RandomSpawnObstacle (Transformation|GetWorldTransform (Variables|Default|GetLaneArrow_1)))))
    (:then_2
      (if (CallFunction|FirstDifficultyCheck)
        (CallFunction|RandomSpawnObstacle (Transformation|GetWorldTransform (Variables|Default|GetLaneArrow_2)))))))

(fn RandomSpawnObstacle
  (params (InTransform :type Transform))
  (switch int (Math|Random|RandomIntegerinRange 1 (Variables|Default|GetMaxRandomObstacleID))
    (:1
      (bind _returnvalue (Game|SpawnActorfromClass "/Game/Blueprints/Invironment/Obstacles/BP_Obst_Bottom.BP_Obst_Bottom_C" InTransform "Undefined" "MultiplyWithRoot" 0 0 :!label _label))
      (Utilities|Array|Add (Variables|Default|GetActors) _returnvalue))
    (:2
      (bind _returnvalue_2 (Game|SpawnActorfromClass "/Game/Blueprints/Invironment/Obstacles/BP_Obst_Top.BP_Obst_Top_C" InTransform "Undefined" "MultiplyWithRoot" 0 0 :!label _label_2))
      (Utilities|Array|Add (Variables|Default|GetActors) _returnvalue_2))
    (:3
      (bind _returnvalue_3 (Game|SpawnActorfromClass "/Game/Blueprints/Invironment/Obstacles/BP_Obst_Vert.BP_Obst_Vert_C" InTransform "Undefined" "MultiplyWithRoot" 0 0))
      (Utilities|Array|Add (Variables|Default|GetActors) _returnvalue_3))
    (:4
      (if (CallFunction|SecondDifficultyCheck 1)
        (goto _label)))
    (:5
      (if (CallFunction|SecondDifficultyCheck 12)
        (goto _label_2)))
    (:6
      (switch int (Math|Random|RandomIntegerinRange 1 (Variables|Default|GetMaxRandomObstacleID))
        (:1
          (bind _returnvalue_4 (Game|SpawnActorfromClass "/Game/Blueprints/Invironment/Bonuses/BP_Bonus_Coin.BP_Bonus_Coin_C" InTransform "Undefined" "MultiplyWithRoot" 0 0))
          (Utilities|Array|Add (Variables|Default|GetActors) _returnvalue_4))
        (:2
          (bind _returnvalue_5 (Game|SpawnActorfromClass "/Game/Blueprints/Invironment/Bonuses/BP_Bonus_SpeedUp.BP_Bonus_SpeedUp_C" InTransform "Undefined" "MultiplyWithRoot" 0 0))
          (Utilities|Array|Add (Variables|Default|GetActors) _returnvalue_5))
        (:3
          (bind _returnvalue_6 (Game|SpawnActorfromClass "/Game/Blueprints/Invironment/Bonuses/BP_Bonus_SpeedDown.BP_Bonus_SpeedDown_C" InTransform "Undefined" "MultiplyWithRoot" 0 0))
          (Utilities|Array|Add (Variables|Default|GetActors) _returnvalue_6))))))

(fn TileEnds
  (Utilities|FlowControl|Sequence
    (:then_0
      (for _array_element (Variables|Default|GetActors)
        (Utilities|IsValid _array_element
          (:Is%20Valid
            (Actor|DestroyActor _array_element)))))
    (:then_1
      (Actor|DestroyActor))))

(fn FirstDifficultyCheck
  (params (InDificulty :type Integer))
  (if (> (Variables|/Game/Blueprints/BP_Gamemode.BP_Gamemode_C|GetCurrentDifficulty (Variables|Default|GetCurrentGamemode)) InDificulty)
    (return true)
    (else
      (return (Math|Random|RandomBool)))))

(fn SecondDifficultyCheck
  (params (InDificulty :type Integer))
  (if (> (Variables|/Game/Blueprints/BP_Gamemode.BP_Gamemode_C|GetCurrentDifficulty (Variables|Default|GetCurrentGamemode)) InDificulty)
    (return (Math|Random|RandomBool))
    (else
      (return false))))