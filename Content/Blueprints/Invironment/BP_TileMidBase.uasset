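; Base middle tile of an endlessly spawned track, with randomized scenery in a right and left volume.
; Construction scatters instanced props from a mesh list in both volumes with random position, rotation and scale.
; BeginPlay spawns a random, randomly yawed house actor at each volume.
; When the player overlaps the exit box, the game mode spawns another tile and updates the count; after a delay, this tile and its houses are destroyed.
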(event OnComponentBeginOverlap(TileExitBoxCollision)
  (params (OverlappedComponent :type Primitive%20Component%20Object%20Reference) (OtherActor :type Actor%20Object%20Reference) (OtherComp :type Primitive%20Component%20Object%20Reference) (OtherBodyIndex :type Integer) (bFromSweep :type Boolean) (SweepResult :type Hit%20Result%20Structure%20%28by%20ref%29))
  (Utilities|Casting|CastToBP_PlayerCharacters OtherActor)
  (bind _asbp_gamemode (Utilities|Casting|CastToBP_Gamemode (Game|GetGameMode)))
  (Default|SpawnMidTile _asbp_gamemode "BP_TileMidBase_C")
  (Default|UpdateTileCount _asbp_gamemode)
  (Utilities|FlowControl|Delay 3.0)
  (for _array_element (Variables|Default|GetSpawnedHouseActors)
    (Actor|DestroyActor _array_element))
  (Actor|DestroyActor))

(event EventBeginPlay
  (Utilities|FlowControl|Sequence
    (:then_0
      (CallFunction|AddHouseBlueprint (Transformation|GetWorldTransform (Variables|Default|GetPropsValumeR))))
    (:then_1
      (CallFunction|AddHouseBlueprint (Transformation|GetWorldTransform (Variables|Default|GetPropsValumeL))))))

(fn ConstructionScript
  (Utilities|FlowControl|Sequence
    (:then_0
      (CallFunction|GenerateProps))))

(fn GenerateProps
  (for (_array_element _array_index) (Variables|Default|GetStaticMeshes)
    (bind _returnvalue (AddComponent|AddInstancedStaticMeshComponent false))
    (LocalVariables|SetL_Instance _returnvalue)
    (bind _returnvalue_2 (Components|StaticMesh|SetStaticMesh (LocalVariables|GetL_Instance) _array_element))
    (if _returnvalue_2
      (for _index (range 1 (Utilities|Array|Get(acopy) (Variables|Default|GetMeshesCount) _array_index))
        (Utilities|FlowControl|Sequence
          (:then_0
            (CallFunction|AddPropsInstance (LocalVariables|GetL_Instance) (Variables|Default|GetPropsValumeR)))
          (:then_1
            (CallFunction|AddPropsInstance (LocalVariables|GetL_Instance) (Variables|Default|GetPropsValumeL))))))))

(fn AddPropsInstance
  (params (InInstance :type Instanced%20Static%20Mesh%20Component%20Object%20Reference) (InValume :type Box%20Component%20Object%20Reference))
  (bind _returnvalue (Math|Random|RandomFloatinRange -5.0 5.0))
  (bind _boxextent (Variables|/Script/Engine.BoxComponent|GetBoxExtent InValume))
  (LocalVariables|SetL_XYScale (Math|Random|RandomFloatinRange 0.8 1.2))
  (LocalVariables|SetL_Rotator (Math|Rotator|MakeRotator _returnvalue _returnvalue (Math|Random|RandomFloatinRange -0.0 3.6e+02)))
  (LocalVariables|SetL_Location (Math|Vector|MakeVector (Math|Random|RandomFloatinRange (* (.x _boxextent) -1.0) (.x _boxextent)) (Math|Random|RandomFloatinRange (* (.y _boxextent) -1.0) (.z _boxextent)) 0.0))
  (Components|InstancedStaticMesh|AddInstance InInstance (Math|Transform|MakeTransform (+ (LocalVariables|GetL_Location) (Variables|/Script/Engine.SceneComponent|GetRelativeLocation InValume)) (LocalVariables|GetL_Rotator) (Math|Vector|MakeVector (LocalVariables|GetL_XYScale) (LocalVariables|GetL_XYScale) (Math|Random|RandomFloatinRange 1.0 1.1))) false))

(fn AddHouseBlueprint
  (params (InSpawnTransform :type Transform))
  (bind (_location _rotation _scale) (Math|Transform|BreakTransform InSpawnTransform))
  (bind (_roll _pitch) (Math|Rotator|BreakRotator _rotation))
  (bind _returnvalue (Game|SpawnActorfromClass (Utilities|Array|Get(acopy) (Variables|Default|GetHouseActors) (Math|Random|RandomIntegerinRange 0 (Utilities|Array|LastIndex (Variables|Default|GetHouseActors)))) (Math|Transform|MakeTransform _location (Math|Rotator|MakeRotator _roll _pitch (Math|Random|RandomFloatinRange 0.0 3.6e+02)) _scale) "Undefined" "MultiplyWithRoot" 0 0))
  (Utilities|Array|Add (Variables|Default|GetSpawnedHouseActors) _returnvalue))