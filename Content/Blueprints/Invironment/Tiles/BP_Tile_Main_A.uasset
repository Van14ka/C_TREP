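; BP_Tile_Main_A is an environment tile Blueprint that randomizes the look of its walls when play begins.
; After the parent BeginPlay, it passes its four left and right wall components to UpdateWallStaticMeshRandom.
; That function sets each component to an independently chosen random entry from the WallStaticMeshes array.
; The randomization runs only at runtime, as the construction script just calls its parent.
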(event EventBeginPlay
  (|CallParentFunction)
  (Utilities|FlowControl|Sequence
    (:then_0
      (CallFunction|UpdateWallStaticMeshRandom (Variables|Default|GetWall_02L)))
    (:then_1
      (CallFunction|UpdateWallStaticMeshRandom (Variables|Default|GetWall_01L)))
    (:then_2
      (CallFunction|UpdateWallStaticMeshRandom (Variables|Default|GetWall_02R)))
    (:then_3
      (CallFunction|UpdateWallStaticMeshRandom (Variables|Default|GetWall_01R)))))

(event Collision|EventActorBeginOverlap
  (params (OtherActor :type Actor%20Object%20Reference)))

(event EventTick
  (params (DeltaSeconds :type Float%20%28single-precision%29)))

(fn ConstructionScript
  (|CallParentFunction))

(fn UpdateWallStaticMeshRandom
  (params (InSMC :type Static%20Mesh%20Component%20Object%20Reference))
  (Components|StaticMesh|SetStaticMesh InSMC (Utilities|Array|Get(acopy) (Variables|Default|GetWallStaticMeshes) (Math|Random|RandomIntegerinRange 0 (Utilities|Array|LastIndex (Variables|Default|GetWallStaticMeshes))))))