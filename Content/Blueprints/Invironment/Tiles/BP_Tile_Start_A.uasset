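; BP_Tile_Start_A is a start tile that replaces the parent's obstacle spawning with decorative spark effects.
; Its SpawnObstacles override never calls the parent version, instead spawning P_Sparks emitters at the LaneArrow0 and LaneArrow2 lane markers.
; The spawned emitters are stored in Particles, and TileEnds runs the parent logic, then destroys each one.
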(event EventBeginPlay)

(event Collision|EventActorBeginOverlap
  (params (OtherActor :type Actor%20Object%20Reference)))

(event EventTick
  (params (DeltaSeconds :type Float%20%28single-precision%29)))

(fn ConstructionScript
  (|CallParentFunction))

(fn SpawnObstacles
  (Utilities|FlowControl|Sequence
    (:then_0
      (bind _returnvalue (Effects|SpawnEmitteratLocation "/Game/StarterContent/Particles/P_Sparks.P_Sparks" (Transformation|GetWorldLocation (Variables|Default|GetLaneArrow_0))))
      (Utilities|Array|Add (Variables|Default|GetParticles) _returnvalue))
    (:then_1
      (bind _returnvalue_2 (Effects|SpawnEmitteratLocation "/Game/StarterContent/Particles/P_Sparks.P_Sparks" (Transformation|GetWorldLocation (Variables|Default|GetLaneArrow_2))))
      (Utilities|Array|Add (Variables|Default|GetParticles) _returnvalue_2))))

(fn TileEnds
  (|CallParentFunction)
  (for _array_element (Variables|Default|GetParticles)
    (Components|DestroyComponent _array_element)))