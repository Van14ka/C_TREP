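; BP_BonusBase is a bonus pickup that awards score when a player character overlaps it.
; On overlap with a BP_PlayerCharacters actor it calls ApplyBonus, plays BonusSound at its location and destroys itself.
; ApplyBonus passes DefaultScore to BP_Gamemode's UpdateScoreSumm.
; A random yaw rotation of the SMCBonus component is left unconnected, so it never runs.
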(event EventBeginPlay)

(event Collision|EventActorBeginOverlap
  (params (OtherActor :type Actor%20Object%20Reference))
  (Utilities|Casting|CastToBP_PlayerCharacters OtherActor)
  (CallFunction|ApplyBonus)
  (Audio|PlaySoundatLocation (Variables|Default|GetBonusSound) (Transformation|GetActorLocation) "0, 0, 0" 1.0 1.0 0.0 0 0 0 0)
  (Actor|DestroyActor))

(event EventTick
  (params (DeltaSeconds :type Float%20%28single-precision%29)))

(fn ConstructionScript)

(fn ApplyBonus
  (bind _asbp_gamemode (Utilities|Casting|CastToBP_Gamemode (Game|GetGameMode)))
  (Default|UpdateScoreSumm _asbp_gamemode (Variables|Default|GetDefaultScore)))