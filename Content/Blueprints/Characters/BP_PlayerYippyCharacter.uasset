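; BP_PlayerYippyCharacter is the player Yippy character, a child Blueprint that extends its parent's begin play and death behavior.
; On BeginPlay it runs the parent logic, then activates its RotatingMovement component without a reset.
; Death runs the parent logic, swaps the mesh's face material to M_Face_25, and calls the same activation on RotatingMovement again.
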(event EventBeginPlay
  (|CallParentFunction)
  (Components|Activation|Activate (Variables|Default|GetRotatingMovement) false))

(event Collision|EventActorBeginOverlap
  (params (OtherActor :type Actor%20Object%20Reference)))

(event EventTick
  (params (DeltaSeconds :type Float%20%28single-precision%29))
  (|CallParentFunction DeltaSeconds) ; This node is disabled and will not be called.\nDrag off pins to build functionality.
)

(fn ConstructionScript)

(fn Death
  (|CallParentFunction)
  (Rendering|Material|SetMaterial (Variables|Character|GetMesh) 1 "/Game/Art/Yippy_Kawaii/Materials/Faces_Materials/M_Face_25.M_Face_25")
  (Components|Activation|Activate (Variables|Default|GetRotatingMovement) false))